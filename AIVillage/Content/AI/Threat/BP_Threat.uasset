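; BP_Threat is a short-lived threat actor that chases NPCs and puts them into a threatened state before destroying itself.
; DetectionSphere overlaps set or clear each NPC's ThreatActor and threat flag through CambiarAmenaza, with a delayed initial scan and cleanup on EndPlay.
; BuscarNPC, presumably run by the looping timer, picks the nearest BP_NPC_Base.
; Tick slides toward that target at constant speed on XY, stopping short of it.
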(event OnComponentBeginOverlap(DetectionSphere)
  (params (OverlappedComponent :type Primitive%20Component%20Object%20Reference) (OtherActor :type Actor%20Object%20Reference) (OtherComp :type Primitive%20Component%20Object%20Reference) (OtherBodyIndex :type Integer) (bFromSweep :type Boolean) (SweepResult :type Hit%20Result%20Structure%20%28by%20ref%29))
  (bind _asbp_npc_base (Utilities|Casting|CastToBP_NPC_Base OtherActor))
  (Variables|/Game/AI/NPC/BP_NPC_Base.BP_NPC_Base_C|SetThreatActor _asbp_npc_base self)
  (Default|CambiarAmenaza _asbp_npc_base true)
  (Development|PrintString "NPC DETECTÓ AMENAZA"))

(event OnComponentEndOverlap(DetectionSphere)
  (params (OverlappedComponent :type Primitive%20Component%20Object%20Reference) (OtherActor :type Actor%20Object%20Reference) (OtherComp :type Primitive%20Component%20Object%20Reference) (OtherBodyIndex :type Integer))
  (bind _asbp_npc_base (Utilities|Casting|CastToBP_NPC_Base OtherActor))
  (if (== self (Variables|/Game/AI/NPC/BP_NPC_Base.BP_NPC_Base_C|GetThreatActor _asbp_npc_base))
    (Default|CambiarAmenaza _asbp_npc_base false)
    (Variables|/Game/AI/NPC/BP_NPC_Base.BP_NPC_Base_C|SetThreatActor _asbp_npc_base 0)
    (Development|PrintString "NPC FUERA DE PELIGRO")))

(event Custom|BuscarNPC
  (Variables|Default|SetObjetivoNPC 0)
  (Variables|Default|SetMejorDistancia 999999.0)
  (bind _outactors (Actor|GetAllActorsOfClass "/Game/AI/NPC/BP_NPC_Base.BP_NPC_Base_C"))
  (for _array_element _outactors
    (if (< (Math|Vector|Distance(Vector) (Transformation|GetActorLocation _array_element) (Transformation|GetActorLocation)) (Variables|Default|GetMejorDistancia))
      (Variables|Default|SetMejorDistancia (Math|Vector|Distance(Vector) (Transformation|GetActorLocation _array_element) (Transformation|GetActorLocation)))
      (Variables|Default|SetObjetivoNPC _array_element)))
  (Utilities|IsValid (Variables|Default|GetObjetivoNPC)
    (:Is%20Valid
      (Development|PrintString "OBJETIVO ENCONTRADO"))
    (:Is%20Not%20Valid
      (Development|PrintString "SIN OBJETIVO"))))

(event EventBeginPlay
  (Utilities|FlowControl|Sequence
    (:then_0
      (Utilities|FlowControl|Delay 0.2)
      (for _array_element (Collision|GetOverlappingActors (Variables|Default|GetDetectionSphere) "/Game/AI/NPC/BP_NPC_Base.BP_NPC_Base_C" :!class /Script/Engine.PrimitiveComponent)
        (bind _asbp_npc_base (Utilities|Casting|CastToBP_NPC_Base _array_element))
        (Variables|/Game/AI/NPC/BP_NPC_Base.BP_NPC_Base_C|SetThreatActor _asbp_npc_base self)
        (Default|CambiarAmenaza _asbp_npc_base true)))
    (:then_1
      (Utilities|Time|SetTimerbyEvent (EventDispatchers|CreateEvent :!event Custom|BuscarNPC) 0.5 true))
    (:then_2
      (Utilities|FlowControl|Delay 15.0)
      (Actor|DestroyActor))))

(event Collision|EventActorBeginOverlap
  (params (OtherActor :type Actor%20Object%20Reference)))

(event EventTick
  (params (DeltaSeconds :type Float%20%28single-precision%29))
  (bind _returnvalue (Transformation|GetActorLocation))
  (bind _objetivonpc (Variables|Default|GetObjetivoNPC))
  (bind _returnvalue_2 (Transformation|GetActorLocation _objetivonpc))
  (bind (_x _y) (Math|Vector|BreakVector _returnvalue_2))
  (Utilities|IsValid _objetivonpc
    (:Is%20Valid
      (if (> (Math|Vector|Distance(Vector) _returnvalue _returnvalue_2) 1.5e+02)
        (Transformation|SetActorLocation (Math|Interpolation|VInterptoConstant _returnvalue (Math|Vector|MakeVector _x _y (.Z (Math|Vector|BreakVector _returnvalue))) DeltaSeconds 2.5e+02) false false)))))

(event EventEndPlay
  (params (EndPlayReason :type EEndPlayReason%20Enum :default "Destroyed"))
  (bind _outactors (Actor|GetAllActorsOfClass "/Game/AI/NPC/BP_NPC_Base.BP_NPC_Base_C"))
  (for _array_element _outactors
    (bind _asbp_npc_base (Utilities|Casting|CastToBP_NPC_Base _array_element))
    (if (== (Variables|/Game/AI/NPC/BP_NPC_Base.BP_NPC_Base_C|GetThreatActor _asbp_npc_base) self)
      (Default|CambiarAmenaza _asbp_npc_base false)
      (Variables|/Game/AI/NPC/BP_NPC_Base.BP_NPC_Base_C|SetThreatActor _asbp_npc_base 0))))

(fn ConstructionScript)