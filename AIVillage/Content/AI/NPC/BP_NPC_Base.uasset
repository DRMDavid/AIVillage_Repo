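; Base village NPC Blueprint that switches a threat state on and off for its AI controller's Blackboard.
; CambiarAmenaza frees any reserved Smart Object slot via LimpiarReserva before setting HasThreat, and on threat end resets fleeing and activity state.
; BeginPlay runs a timed test that raises the threat after a delay and clears it after another, with debug prints throughout.
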(event Custom|CambiarAmenaza
  (params (NuevaAmenaza :type Boolean))
  (if NuevaAmenaza
    (bind _liberacioncorrecta (CallFunction|LimpiarReserva))
    (if _liberacioncorrecta
      (Variables|Default|SetHasThreat true)
      (bind _asaic_npc_village (Utilities|Casting|CastToAIC_NPC_Village (Pawn|GetController)))
      (AI|Components|Blackboard|SetValueasBool (Variables|/Script/AIModule.AIController|GetBlackboard _asaic_npc_village) (Utilities|Name|MakeLiteralName "HasThreat") true)
      (Development|PrintString "AMENAZA ACTIVADA")
      (else
        (Development|PrintString "ERROR - AI Controller no encontrado")))
    (else
      (Variables|Default|SetHasThreat false)
      (Variables|Default|SetIsFleeing false)
      (Variables|Default|SetCurrentActivity "NewEnumerator0")
      (bind _asaic_npc_village_2 (Utilities|Casting|CastToAIC_NPC_Village (Pawn|GetController)))
      (AI|Components|Blackboard|SetValueasBool (Variables|/Script/AIModule.AIController|GetBlackboard _asaic_npc_village_2) (Utilities|Name|MakeLiteralName "HasThreat") false)
      (Development|PrintString "AMENAZA TERMINADA"))))

(event EventBeginPlay
  (Utilities|FlowControl|Delay 8.0)
  (CallFunction|CambiarAmenaza true)
  (Utilities|FlowControl|Delay 8.0)
  (CallFunction|CambiarAmenaza false))

(event Collision|EventActorBeginOverlap
  (params (OtherActor :type Actor%20Object%20Reference)))

(event EventTick
  (params (DeltaSeconds :type Float%20%28single-precision%29)))

(fn ConstructionScript)

(fn LimpiarReserva
  (if (Variables|Default|GetHasReservation)
    (bind _returnvalue (Class|SmartObjectBlueprintFunctionLibrary|MarkSmartObjectSlotasFree (Variables|Default|GetReservaActual)))
    (if _returnvalue
      (Variables|Default|SetHasReservation false)
      (Variables|Default|SetIsUsingObject false)
      (Variables|Default|SetCurrentActivity "NewEnumerator0")
      (Variables|Default|SetReservaActual "")
      (Development|PrintString "Reserva limpiada correctamente" true true "(R=0.137981,G=1.000000,B=0.000000,A=1.000000)")
      (return true)
      (else
        (Development|PrintString "ERROR: No se pudo liberar el Slot" true true "(R=1.000000,G=0.000000,B=0.091731,A=1.000000)")
        (return false)))
    (else
      (Development|PrintString "No habia reserva que liberar" true true "(R=1.000000,G=0.000000,B=0.091731,A=1.000000)")
      (return true))))