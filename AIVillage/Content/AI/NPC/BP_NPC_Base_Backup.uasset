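; Base NPC Blueprint, apparently a backup, that sends the NPC to work at a nearby Smart Object on BeginPlay.
; It claims the first slot found, retrying if none, and proceeds only for forge or farm owners.
; After AIMoveTo it occupies the slot, replaces CurrentActivity with PreferredActivity, prints placeholder work and waits before releasing.
; It never searches again after release, and other object types leave the claim held.
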(event Custom|BuscarYUsarForja
  (bind _returnvalue (Transformation|GetActorLocation))
  ;[1 0 0.09567 0.5] Forge
  (bind _outresults (Class|SmartObjectSubsystem|FindSmartObjectsBP (Subsystems|GetSmartObjectSubsystem) (Utilities|Struct|MakeSmartObjectRequest (Math|Box|MakeBox (- _returnvalue "2000.000000,2000.000000,500.000000") (+ _returnvalue "2000.000000,2000.000000,500.000000")) "(UserTags=(GameplayTags=),ClaimPriority=Normal,ActivityRequirements=(TokenStreamVersion=0,TagDictionary=,QueryTokenStream=,UserDescription=\"\",AutoDescription=\"\"),BehaviorDefinitionClasses=,bShouldEvaluateConditions=True,bShouldIncludeClaimedSlots=False,bShouldIncludeDisabledSlots=False)") self))
  (if (> (Utilities|Array|Length _outresults) 0)
    (bind _returnvalue_2 (Class|SmartObjectBlueprintFunctionLibrary|MarkSmartObjectSlotasClaimed (.slothandle (Utilities|Array|Get(acopy) _outresults)) self "Normal"))
    (Variables|Default|SetReservaActual _returnvalue_2)
    (Development|PrintString (Utilities|GetDisplayName (Components|GetOwner (Class|SmartObjectSubsystem|GetSmartObjectComponent (Subsystems|GetSmartObjectSubsystem) (Variables|Default|GetReservaActual) "No"))))
    (Utilities|Casting|CastToBP_SO_Forge (Components|GetOwner (Class|SmartObjectSubsystem|GetSmartObjectComponent (Subsystems|GetSmartObjectSubsystem) (Variables|Default|GetReservaActual) "No"))
      (:then
        (Variables|Default|SetCurrentActivity "NewEnumerator1"))
      (:CastFailed
        (Utilities|Casting|CastToBP_SO_Farm (Components|GetOwner (Class|SmartObjectSubsystem|GetSmartObjectComponent (Subsystems|GetSmartObjectSubsystem) (Variables|Default|GetReservaActual) "No")))
        (Variables|Default|SetCurrentActivity "NewEnumerator2")))
    (if (.ReturnValue (Class|SmartObjectSubsystem|GetSlotLocation (Subsystems|GetSmartObjectSubsystem) (Variables|Default|GetReservaActual)))
      (AI|AIMoveTo self (.OutSlotLocation (Class|SmartObjectSubsystem|GetSlotLocation (Subsystems|GetSmartObjectSubsystem) (Variables|Default|GetReservaActual))) 0 1e+01 false
        (:OnSuccess
          (bind _returnvalue_3 (Class|SmartObjectBlueprintFunctionLibrary|MarkSmartObjectSlotasOccupied (Variables|Default|GetReservaActual) "/Script/GameplayBehaviorSmartObjectsModule.GameplayBehaviorSmartObjectBehaviorDefinition"))
          (if (Utilities|IsValid _returnvalue_3)
            (bind _output_get (Variables|Default|SetCurrentActivity (Variables|Default|GetPreferredActivity)))
            (switch Utilities|FlowControl|Switch|SwitchonE_NPC_Activity _output_get
              (:NewEnumerator1
                (Development|PrintString "Trabajando en la forja")
                (Utilities|FlowControl|Delay 4.0)
                (CallFunction|LiberarReserva))
              (:NewEnumerator2
                (Development|PrintString "Trabajando en la Granja")
                (Utilities|FlowControl|Delay 4.0)
                (CallFunction|LiberarReserva))
              (:NewEnumerator3
                (Development|PrintString "Trabajando en el Pozo")
                (Utilities|FlowControl|Delay 4.0)
                (CallFunction|LiberarReserva))
              (:NewEnumerator4
                (Development|PrintString "Descansando")
                (Utilities|FlowControl|Delay 4.0)
                (CallFunction|LiberarReserva))
              (:NewEnumerator5
                (Development|PrintString "Huir")
                (Utilities|FlowControl|Delay 4.0)
                (CallFunction|LiberarReserva)))
            (else
              (Development|PrintString "Print String: Error al ocupar Slot")
              (CallFunction|LiberarReserva))))
        (:OnFail
          (Development|PrintString "¡AI Falló!")
          (CallFunction|LiberarReserva)))
      (else
        (Development|PrintString "Slot sin ubicación")))
    (else
      (Development|PrintString "No hay Slots disponibles")
      (Utilities|FlowControl|Delay 2.0)
      (CallFunction|BuscarYUsarForja))))

(event Custom|LiberarReserva
  ;[1 0 0.09567 0.5] Forge
  (bind _returnvalue (Class|SmartObjectBlueprintFunctionLibrary|MarkSmartObjectSlotasFree (Variables|Default|GetReservaActual)))
  (if _returnvalue
    (Variables|Default|SetCurrentActivity "NewEnumerator0")
    (Development|PrintString "Slot liberado correctamente")
    (else
      (Development|PrintString "ERROR: No se pudo liberar el Slot"))))

(event EventBeginPlay
  ;[1 0 0.09567 0.5] Forge
  (CallFunction|BuscarYUsarForja))

(event Collision|EventActorBeginOverlap
  (params (OtherActor :type Actor%20Object%20Reference)))

(event EventTick
  (params (DeltaSeconds :type Float%20%28single-precision%29)))

(fn ConstructionScript)