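; BP_Threat is an actor that marks nearby NPCs as threatened.
; Shortly after BeginPlay it calls CambiarAmenaza(true) on every overlapping BP_NPC_Base, catching NPCs that start inside its area.
; After that, DetectionSphere begin and end overlaps set the threat state on or off for each NPC and print Spanish debug messages.
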(event OnComponentBeginOverlap(DetectionSphere)
  (params (OverlappedComponent :type Primitive%20Component%20Object%20Reference) (OtherActor :type Actor%20Object%20Reference) (OtherComp :type Primitive%20Component%20Object%20Reference) (OtherBodyIndex :type Integer) (bFromSweep :type Boolean) (SweepResult :type Hit%20Result%20Structure%20%28by%20ref%29))
  (bind _asbp_npc_base (Utilities|Casting|CastToBP_NPC_Base OtherActor))
  (Default|CambiarAmenaza _asbp_npc_base true)
  (Development|PrintString "NPC DETECTÓ AMENAZA"))

(event OnComponentEndOverlap(DetectionSphere)
  (params (OverlappedComponent :type Primitive%20Component%20Object%20Reference) (OtherActor :type Actor%20Object%20Reference) (OtherComp :type Primitive%20Component%20Object%20Reference) (OtherBodyIndex :type Integer))
  (bind _asbp_npc_base (Utilities|Casting|CastToBP_NPC_Base OtherActor))
  (Default|CambiarAmenaza _asbp_npc_base false)
  (Development|PrintString "NPC FUERA DE PELIGRO"))

(event EventBeginPlay
  (Utilities|FlowControl|Delay 0.2)
  (for _array_element (Collision|GetOverlappingActors "/Game/AI/NPC/BP_NPC_Base.BP_NPC_Base_C" :!class /Script/Engine.Actor)
    (bind _asbp_npc_base (Utilities|Casting|CastToBP_NPC_Base _array_element))
    (Default|CambiarAmenaza _asbp_npc_base true)))

(event Collision|EventActorBeginOverlap
  (params (OtherActor :type Actor%20Object%20Reference)))

(event EventTick
  (params (DeltaSeconds :type Float%20%28single-precision%29)))

(fn ConstructionScript)